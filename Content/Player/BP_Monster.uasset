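; BP_Monster is a damageable monster actor that explodes when its health runs out.
; AnyDamage subtracts the incoming damage from an integer HP, truncating the result, and prints the new value to screen.
; At zero or below, it spawns the P_Explosion particle emitter at its location and destroys itself.
; BeginPlay, overlap, Tick and the construction script contain no logic.
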(event `self.ReceiveAnyDamage`
  (params (Damage :type "Float (single-precision)") (DamageType :type "DamageType Object Reference") (InstigatedBy :type "Controller Object Reference") (DamageCauser :type "Actor Object Reference"))
  (bind _output_get (set `self.HP` (`KismetMathLibrary.FTrunc` (- (`self.HP`) Damage))))
  (`KismetSystemLibrary.PrintString` (`KismetStringLibrary.Conv_IntToString` _output_get))
  (if (<= _output_get 0)
    (`GameplayStatics.SpawnEmitterAtLocation` "/Game/StarterContent/Particles/P_Explosion.P_Explosion" (`self.K2_GetActorLocation`))
    (`self.K2_DestroyActor`)))

(fn `UserConstructionScript`)